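; Lens changer actor that toggles red, green and blue lenses to tint the scene and reveal color-matched puzzle objects.
; Each color event adds or removes its color in a stack, then the HUD updates and the directional light takes the summed color, white when empty.
; Every BP_PuzzleObject becomes visible on an exact color match; otherwise it turns translucent under white light, or invisible under any other color.
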(event `self.ReceiveBeginPlay`
  (`LightComponent.SetLightColor` (`Light.LightComponent` (`self.directionalLight`)) (`self.WhiteColor`) true))

(event `Red`
  (bind _colorstack (`self.colorStack`))
  (bind _returnvalue (`KismetArrayLibrary.Array_AddUnique` _colorstack (`self.RedColor`)))
  (if (< _returnvalue 0)
    (`KismetArrayLibrary.Array_RemoveItem` _colorstack (`self.RedColor`)))
  (`self.OnColorChange`))

(event `Green`
  (bind _colorstack (`self.colorStack`))
  (bind _returnvalue (`KismetArrayLibrary.Array_AddUnique` _colorstack (`self.GreenColor`)))
  (if (< _returnvalue 0)
    (`KismetArrayLibrary.Array_RemoveItem` _colorstack (`self.GreenColor`)))
  (`self.OnColorChange`))

(event `Blue`
  (bind _colorstack (`self.colorStack`))
  (bind _returnvalue (`KismetArrayLibrary.Array_AddUnique` _colorstack (`self.BlueColor`)))
  (if (< _returnvalue 0)
    (`KismetArrayLibrary.Array_RemoveItem` _colorstack (`self.BlueColor`)))
  (`self.OnColorChange`))

(event `OnColorChange`
  (bind _asbp_hud (cast `/Game/UI/Blueprints/BP_HUD` (`PlayerController.GetHUD` (`GameplayStatics.GetPlayerController` 0))))
  (`/Game/UI/Blueprints/BP_HUD.OnColorChangeHUDEvent` _asbp_hud (`self.colorStack`))
  (bind _resultantcolorout (`self.getResultantColor`))
  (`LightComponent.SetLightColor` (`Light.LightComponent` (`self.directionalLight`)) _resultantcolorout true)
  (bind _outactors (`GameplayStatics.GetAllActorsOfClass` "/Game/Blueprints/BP_PuzzleObject.BP_PuzzleObject_C"))
  (for _array_element _outactors
    (if (== (`/Game/Blueprints/BP_PuzzleObject.color` _array_element) _resultantcolorout)
      (`/Game/Blueprints/BP_PuzzleObject.makeVisible` _array_element)
      (elif (== _resultantcolorout (`self.WhiteColor`))
        (`/Game/Blueprints/BP_PuzzleObject.Make Translucent` _array_element)
        (else
          (`/Game/Blueprints/BP_PuzzleObject.makeInvisible` _array_element))))))

(fn `getResultantColor`
  (returns (resultantColorOut :type "LinearColor Structure"))
  (locals (resultantColor :type "LinearColor Structure" :default (struct)))
  (for _array_element (`self.colorStack`)
    (bind _output_get (set `local.resultantColor` (+ _array_element (`local.resultantColor`)))))
  (bind (_r _g _b) (break `LinearColor` (select `bool` (`KismetArrayLibrary.Array_IsEmpty` (`self.colorStack`)) :`false` _output_get :`true` (struct :`R` 1.0 :`G` 1.0 :`B` 1.0 :`A` 1.0))))
  (return (make `LinearColor` _r _g _b 1.0)))

(fn `UserConstructionScript`)