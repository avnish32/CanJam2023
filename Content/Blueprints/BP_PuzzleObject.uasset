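; BP_PuzzleObject is a puzzle actor whose static mesh switches between translucent non-colliding, opaque solid and hidden states.
; BeginPlay creates translucent and opaque dynamic material instances for tinting, then starts the object translucent.
; Visibility functions swap material, collision or mesh visibility to change state.
; If movable, it ping-pongs on Tick between two positions at constant speed from a travel time, swapping endpoints on arrival.
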(event `self.ReceiveBeginPlay`
  (`self.instantiateTranslucentMaterialInstance`)
  (`self.instantiateOpaqueMaterialInstance`)
  (`self.Make Translucent`)
  (if (`self.isMovable`)
    (`self.K2_SetActorLocation` (`self.Pos1`))))

(event `self.ReceiveTick`
  (params (DeltaSeconds :type "Float (single-precision)"))
  (if (`self.isMovable`)
    (`self.MoveObject`)))

(fn `instantiateOpaqueMaterialInstance`
  (`self.opaqueMaterialInstance`
    (:`then`
      _)
    (:`else`
      (bind _returnvalue (`KismetMaterialLibrary.CreateDynamicMaterialInstance` "/Game/Materials/M_ObjectOpaque.M_ObjectOpaque"))
      (bind _output_get (set `self.opaqueMaterialInstance` _returnvalue))))
  (`MaterialInstanceDynamic.SetVectorParameterValue` _output_get "None" (`self.color`)))

(fn `instantiateTranslucentMaterialInstance`
  (bind _translucentmaterialinstance (`self.translucentMaterialInstance`)
    (:`then`
      _)
    (:`else`
      (bind _returnvalue (`PrimitiveComponent.CreateDynamicMaterialInstance` (`self.StaticMesh`) 0 "/Game/Materials/M_ObjectTranslucent.M_ObjectTranslucent" "None"))
      (bind _output_get (set `self.translucentMaterialInstance` _returnvalue))))
  (`MaterialInstanceDynamic.SetVectorParameterValue` _output_get "Color" (`self.color`))
  (`MaterialInstanceDynamic.SetVectorParameterValue` _translucentmaterialinstance "Color" (`self.color`)))

(fn `Make Translucent`
  (bind _staticmesh (`self.StaticMesh`))
  (`PrimitiveComponent.SetCollisionEnabled` _staticmesh "NoCollision")
  (`PrimitiveComponent.SetMaterial` _staticmesh 0 (`self.translucentMaterialInstance`))
  (`SceneComponent.SetVisibility` _staticmesh true false))

(fn `makeInvisible`
  (bind _staticmesh (`self.StaticMesh`))
  (`PrimitiveComponent.SetCollisionEnabled` _staticmesh "NoCollision")
  (`SceneComponent.SetVisibility` _staticmesh false false))

(fn `makeVisible`
  (bind _staticmesh (`self.StaticMesh`))
  (`PrimitiveComponent.SetCollisionEnabled` _staticmesh "QueryAndPhysics")
  (`PrimitiveComponent.SetMaterial` _staticmesh 0 (`self.opaqueMaterialInstance`))
  (`SceneComponent.SetVisibility` _staticmesh true false))

(fn `MoveObject`
  (locals (tempPosition :type "Vector Structure"))
  (`self.K2_SetActorLocation` (`KismetMathLibrary.VInterpTo_Constant` (`self.K2_GetActorLocation`) (`self.Pos2`) (`GameplayStatics.GetWorldDeltaSeconds`) (/ (`KismetMathLibrary.Vector_Distance` (`self.Pos1`) (`self.Pos2`)) (`self.timeFromPos1To2`))))
  (if (== (`self.K2_GetActorLocation`) (`self.Pos2`) :`ErrorTolerance` 0.1)
    (set `local.tempPosition` (`self.Pos2`))
    (set `self.Pos2` (`self.Pos1`))
    (set `self.Pos1` (`local.tempPosition`))))

(fn `toggleVisibility`
  (bind _staticmesh (`self.StaticMesh`))
  (bind _isvisible (`self.isVisible`))
  (`PrimitiveComponent.SetCollisionEnabled` _staticmesh (select `bool` _isvisible :`false` "QueryAndPhysics" :`true` "NoCollision" :!type "ECollisionEnabled Enum"))
  (`PrimitiveComponent.SetMaterial` _staticmesh 0 (select `bool` _isvisible :`false` (`self.opaqueMaterialInstance`) :`true` (`self.translucentMaterialInstance`) :!type "MaterialInterface Object Reference"))
  (set `self.isVisible` (not (`self.isVisible`))))

(fn `UserConstructionScript`)