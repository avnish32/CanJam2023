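; Game mode for the epilogue level that shows a sequence of story messages and then returns to the main menu.
; On BeginPlay it views through the level's camera actor, builds a bottom-centered text widget on a canvas and switches input to UI only.
; A delay loop advances through the EpilogueMsgs array every few seconds.
; On the last message it reveals a Main Menu button that opens the MenuAndStory level.
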(event `self.ReceiveBeginPlay`
  (bind _returnvalue (`GameplayStatics.GetPlayerController` 0))
  (bind _epiloguemsgwidget (`self.epilogueMsgWidget`))
  (bind _epiloguemsgwidget_2 (`self.epilogueMsgWidget`))
  (bind _returnvalue_2 (`GameplayStatics.GetActorOfClass` "/Script/Engine.CameraActor"))
  (`PlayerController.SetViewTargetWithBlend` (`GameplayStatics.GetPlayerController` 0) _returnvalue_2 0.0 "VTBlend_Linear" 0.0 false)
  (bind _returnvalue_3 (`|CreateWidget` "/Game/UI/Blueprints/BP_TutorialParentWidget.BP_TutorialParentWidget_C"))
  (`UserWidget.AddToViewport` _returnvalue_3 0)
  (set `self.parentCanvas` (`/Game/UI/Blueprints/BP_TutorialParentWidget.CanvasPanel` _returnvalue_3))
  (bind _returnvalue_4 (`|CreateWidget` "/Game/UI/Blueprints/BP_TextWithButton.BP_TextWithButton_C"))
  (set `self.epilogueMsgWidget` _returnvalue_4)
  (`Widget.SetVisibility` (`/Game/UI/Blueprints/BP_TextWithButton.Button_103` _returnvalue_4) "Hidden")
  (bind _returnvalue_5 (`CanvasPanel.AddChildToCanvas` (`self.parentCanvas`) _returnvalue_4))
  (`CanvasPanelSlot.SetAnchors` _returnvalue_5 (make `Anchors` (0.5 1.0) (0.5 1.0)))
  (`CanvasPanelSlot.SetAlignment` _returnvalue_5 (0.5 1.0))
  (set `CanvasPanelSlot.bAutoSize` true _returnvalue_5)
  (`WidgetBlueprintLibrary.SetInputMode_UIOnlyEx` _returnvalue (`self.epilogueMsgWidget`))
  (set `PlayerController.bShowMouseCursor` true _returnvalue)
  (set `TextBlock.Text` (`|GetArrayItem` (`self.epilogueMsgs`) (`self.epilogueMsgsIndex`)) (`/Game/UI/Blueprints/BP_TextWithButton.TextBlock` (`self.epilogueMsgWidget`)) :!label _label)
  (if (== (`self.epilogueMsgsIndex`) (- (`KismetArrayLibrary.Array_Length` (`self.epilogueMsgs`)) 1))
    (`Widget.SetVisibility` (`/Game/UI/Blueprints/BP_TextWithButton.Button_103` _epiloguemsgwidget) "Visible")
    (set `TextBlock.Text` "Main Menu" (`/Game/UI/Blueprints/BP_TextWithButton.buttonText` _epiloguemsgwidget))
    (clear `/Game/UI/Blueprints/BP_TextWithButton.onNextButtonClick` _epiloguemsgwidget_2)
    (add `/Game/UI/Blueprints/BP_TextWithButton.onNextButtonClick` _epiloguemsgwidget_2 (delegate `EpilogueEndButtonClicked`))
    (else
      (`KismetSystemLibrary.Delay` 5.0)
      (`/Engine/EditorBlueprintResources/StandardMacros.IncrementInt` (`self.epilogueMsgsIndex`)
        (:`  `
          (goto _label))))))

(event `EpilogueEndButtonClicked`
  (`GameplayStatics.OpenLevel` "MenuAndStory"))

(fn `UserConstructionScript`)