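; Tutorial game mode that shows a series of text messages in a UI overlay at game start.
; On BeginPlay it switches to UI-only input and anchors a text-and-button widget bottom-centre inside a parent canvas widget.
; Each button click advances through TutorialMsgs until the list runs out, then relabels the button "Play" and rebinds it to EndTutorial.
; EndTutorial restores game-only input, hides the cursor and removes the message widget.
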(event `self.ReceiveBeginPlay`
  (bind _returnvalue (`GameplayStatics.GetPlayerController` 0))
  (`WidgetBlueprintLibrary.SetInputMode_UIOnlyEx` _returnvalue null)
  (set `PlayerController.bShowMouseCursor` true _returnvalue)
  (bind _returnvalue_2 (`|CreateWidget` "/Game/UI/Blueprints/BP_TutorialParentWidget.BP_TutorialParentWidget_C"))
  (set `self.tutorialParentWidget` _returnvalue_2)
  (bind _returnvalue_3 (`|CreateWidget` "/Game/UI/Blueprints/BP_TextWithButton.BP_TextWithButton_C"))
  (bind _output_get (set `self.textWithButtonWidget` _returnvalue_3))
  (add `/Game/UI/Blueprints/BP_TextWithButton.onNextButtonClick` _output_get (delegate `DisplayNextTutorialMsg`))
  (set `TextBlock.Text` (`|GetArrayItem` (`self.tutorialMsgs`)) (`/Game/UI/Blueprints/BP_TextWithButton.TextBlock` _output_get))
  (bind _returnvalue_4 (`CanvasPanel.AddChildToCanvas` (`/Game/UI/Blueprints/BP_TutorialParentWidget.CanvasPanel` (`self.tutorialParentWidget`)) (`self.textWithButtonWidget`)))
  (set `CanvasPanelSlot.bAutoSize` true _returnvalue_4)
  (`CanvasPanelSlot.SetAnchors` _returnvalue_4 (make `Anchors` (0.5 1.0) (0.5 1.0)))
  (`CanvasPanelSlot.SetAlignment` _returnvalue_4 (0.5 1.0))
  (`UserWidget.AddToViewport` (`self.tutorialParentWidget`) 0))

(event `DisplayNextTutorialMsg`
  (bind _textwithbuttonwidget (`self.textWithButtonWidget`))
  (bind _tutorialmsgs (`self.tutorialMsgs`))
  (bind _result (`/Engine/EditorBlueprintResources/StandardMacros.IncrementInt` (`self.tutorialMsgIndex`))
    (:`  `
      (if (== _result (`KismetArrayLibrary.Array_Length` _tutorialmsgs))
        (set `TextBlock.Text` "Play" (`/Game/UI/Blueprints/BP_TextWithButton.buttonText` (`self.textWithButtonWidget`)))
        (clear `/Game/UI/Blueprints/BP_TextWithButton.onNextButtonClick` _textwithbuttonwidget)
        (add `/Game/UI/Blueprints/BP_TextWithButton.onNextButtonClick` _textwithbuttonwidget (delegate `EndTutorial`))
        (else
          (set `TextBlock.Text` (`|GetArrayItem` _tutorialmsgs _result) (`/Game/UI/Blueprints/BP_TextWithButton.TextBlock` (`self.textWithButtonWidget`))))))))

(event `EndTutorial`
  (bind _returnvalue (`GameplayStatics.GetPlayerController` 0))
  (`WidgetBlueprintLibrary.SetInputMode_GameOnly` _returnvalue)
  (set `PlayerController.bShowMouseCursor` false _returnvalue)
  (`Widget.RemoveFromParent` (`self.textWithButtonWidget`)))

(fn `UserConstructionScript`)